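; Actor Blueprint that spins its static mesh around the yaw axis from BeginPlay.
; The Rotation timeline's update adds the reciprocal of RotationAmount360n to the mesh's world yaw on each call and writes it as relative rotation, zeroing roll and pitch.
; The step ignores delta time, and the timeline restart logic is left unconnected.
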(event `self.ReceiveBeginPlay`
  (bind _staticmeshcomponent (`self.StaticMeshComponent`))
  (bind (_returnvalue_roll _returnvalue_pitch _returnvalue_yaw) (`KismetMathLibrary.BreakRotator` (`SceneComponent.K2_GetComponentRotation` _staticmeshcomponent)))
  (`Timeline|Rotation`
    (:`Update`
      (`SceneComponent.K2_SetRelativeRotation` _staticmeshcomponent (`KismetMathLibrary.MakeRotator` 0.0 0.0 (+ _returnvalue_yaw (/ 1.0 (`KismetMathLibrary.Conv_IntToDouble` (`self.Rotation Amount (360/n)`))))) false false))))

(event `self.ReceiveTick`
  (params (DeltaSeconds :type "Float (single-precision)")))

(fn `UserConstructionScript`)