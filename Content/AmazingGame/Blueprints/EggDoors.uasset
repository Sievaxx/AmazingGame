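; EggDoors is a door that opens once the player has collected enough points.
; On BeginPlay it writes PointsNeeded onto two text renders.
; On a hit from a component named "CollisionCylinder", matched by string, it compares player 0's PointsNumber from SourcePlayerChracter against that requirement.
; If met, it disables the mesh's collision, hides it with its children and plays the Eggdoor sound, without deducting points.
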(event `self.ReceiveBeginPlay`
  (`TextRenderComponent.K2_SetText` (`self.TextRender`) (`KismetTextLibrary.Conv_IntToText` (`self.PointsNeeded`)))
  (`TextRenderComponent.K2_SetText` (`self.TextRender1`) (`KismetTextLibrary.Conv_IntToText` (`self.PointsNeeded`))))

(event `self.ReceiveHit`
  (params (MyComp :type "PrimitiveComponent Object Reference") (Other :type "Actor Object Reference") (OtherComp :type "PrimitiveComponent Object Reference") (bSelfMoved :type Boolean) (HitLocation :type "Vector Structure") (HitNormal :type "Vector Structure") (NormalImpulse :type "Vector Structure") (Hit :type "HitResult Structure (by ref)"))
  (bind _staticmeshcomponent (`self.StaticMeshComponent`))
  (if (`KismetStringLibrary.EqualEqual_StrStr` (`KismetStringLibrary.Conv_ObjectToString` OtherComp) "CollisionCylinder")
    (bind _assource_player_chracter (cast `/Game/AmazingGame/Blueprints/SourcePlayerChracter` (`GameplayStatics.GetPlayerCharacter` 0)))
    (if (>= (`/Game/AmazingGame/Blueprints/SourcePlayerChracter.Points Number` _assource_player_chracter) (`self.PointsNeeded`))
      (`PrimitiveComponent.SetCollisionEnabled` _staticmeshcomponent "NoCollision")
      (`SceneComponent.SetVisibility` _staticmeshcomponent false true)
      (`GameplayStatics.PlaySoundAtLocation` "/Game/AmazingGame/Audio/eggdoor.eggdoor" (`self.K2_GetActorLocation`) (struct) 1.0 1.0 0.0 null null null))))

(fn `UserConstructionScript`)