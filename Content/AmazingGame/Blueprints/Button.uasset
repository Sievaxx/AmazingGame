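; Interactive button actor that shows red when idle and turns green with a switch sound for a few seconds when enabled.
; Overlap begin and end toggle the prompt, flip the player character's URGHEnable flag and call the Buttontrue or Buttonfalse dispatcher.
; Tick polls Enabled, which this graph never sets true, and uses AlreadyEnabled to ignore retriggers until the delayed reset to red.
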(event `self.ReceiveBeginPlay`
  (bind _returnvalue (`KismetMathLibrary.MakeColor` 1.0))
  (`MeshComponent.SetVectorParameterValueOnMaterials` (`self.Cube`) "DIffuseColor" (`KismetMathLibrary.Conv_LinearColorToVector` _returnvalue))
  (`TextRenderComponent.SetTextRenderColor` (`self.Prompt`) (`KismetMathLibrary.Conv_LinearColorToColor` _returnvalue)))

(event `self.ReceiveActorBeginOverlap`
  (params (OtherActor :type "Actor Object Reference"))
  (bind _returnvalue (`GameplayStatics.GetPlayerCharacter` 0))
  (bind _prompt (`self.Prompt`))
  (set `self.Interact` true)
  (if (`self.Interact`) :!label _label
    (`SceneComponent.ToggleVisibility` _prompt false)
    (bind _assource_player_chracter (cast `/Game/AmazingGame/Blueprints/SourcePlayerChracter` _returnvalue))
    (set `/Game/AmazingGame/Blueprints/SourcePlayerChracter.URGH_Enable` false _assource_player_chracter)
    (`self.Buttontrue`)
    (else
      (`SceneComponent.ToggleVisibility` _prompt false)
      (bind _assource_player_chracter_2 (cast `/Game/AmazingGame/Blueprints/SourcePlayerChracter` _returnvalue))
      (set `/Game/AmazingGame/Blueprints/SourcePlayerChracter.URGH_Enable` true _assource_player_chracter_2)
      (`self.Buttonfalse`))))

(event `self.ReceiveActorEndOverlap`
  (params (OtherActor :type "Actor Object Reference"))
  (set `self.Interact` false)
  (goto _label))

(event `self.ReceiveTick`
  (params (DeltaSeconds :type "Float (single-precision)"))
  (bind _returnvalue (`KismetMathLibrary.MakeColor` 0.0 1.0))
  (bind _returnvalue_2 (`self.K2_GetActorLocation`))
  (bind _returnvalue_3 (`KismetMathLibrary.MakeColor` 1.0))
  (bind _cube (`self.Cube`))
  (bind _prompt (`self.Prompt`))
  (if (`self.AlreadyEnabled`)
    (set `self.Enabled` false)
    (elif (`self.Enabled`)
      (set `self.AlreadyEnabled` true)
      (set `self.Enabled` false)
      (`MeshComponent.SetVectorParameterValueOnMaterials` _cube "DIffuseColor" (`KismetMathLibrary.Conv_LinearColorToVector` _returnvalue))
      (`TextRenderComponent.SetTextRenderColor` _prompt (`KismetMathLibrary.Conv_LinearColorToColor` _returnvalue))
      (`GameplayStatics.PlaySoundAtLocation` "/Game/AmazingGame/Audio/DSSWTCHN.DSSWTCHN" _returnvalue_2 (struct) 1.0 1.0 0.0 "/Game/AmazingGame/Audio/RealAttenuation.RealAttenuation" null null)
      (`KismetSystemLibrary.Delay` 4.0)
      (`MeshComponent.SetVectorParameterValueOnMaterials` _cube "DIffuseColor" (`KismetMathLibrary.Conv_LinearColorToVector` _returnvalue_3))
      (`TextRenderComponent.SetTextRenderColor` _prompt (`KismetMathLibrary.Conv_LinearColorToColor` _returnvalue_3))
      (`GameplayStatics.PlaySoundAtLocation` "/Game/AmazingGame/Audio/DSSWTCHX.DSSWTCHX" _returnvalue_2 (struct) 1.0 1.0 0.0 "/Game/AmazingGame/Audio/RealAttenuation.RealAttenuation" null null)
      (set `self.AlreadyEnabled` false))))

(fn `UserConstructionScript`)