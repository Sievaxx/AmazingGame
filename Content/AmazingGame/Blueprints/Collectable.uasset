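; Collectable egg pickup that awards the player a point when an actor overlaps it.
; The first overlap hides its sphere, sets a collected flag, adds one to the player character's point count and plays a magic sound at the player.
; After a short delay it plays an egg-get sound and sets the EggGet flag on the first-person HUD.
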(event `self.ReceiveActorBeginOverlap`
  (params (OtherActor :type "Actor Object Reference"))
  (if (not (`self.Collected`))
    (`SceneComponent.SetVisibility` (`self.Sphere`) false false)
    (set `self.Collected` true)
    (bind _assource_player_chracter (cast `/Game/AmazingGame/Blueprints/SourcePlayerChracter` (`GameplayStatics.GetPlayerCharacter` 0)))
    (set `/Game/AmazingGame/Blueprints/SourcePlayerChracter.Points Number` (+ (`/Game/AmazingGame/Blueprints/SourcePlayerChracter.Points Number` _assource_player_chracter) 1) _assource_player_chracter)
    (bind _returnvalue (`self.K2_GetActorLocation` _assource_player_chracter))
    (`GameplayStatics.PlaySoundAtLocation` "/Game/AmazingGame/Audio/magic.magic" _returnvalue (struct) 1.0 1.0 0.0 null null null)
    (`KismetSystemLibrary.Delay` 0.6)
    (`GameplayStatics.PlaySoundAtLocation` "/Game/AmazingGame/Audio/get_egg.get_egg" _returnvalue (struct) 1.0 1.0 0.0 null null null)
    (bind _asfirst_person_hud (cast `/Game/AmazingGame/Blueprints/FirstPersonHUD` (`PlayerController.GetHUD` (`GameplayStatics.GetPlayerController` 0))))
    (set `/Game/AmazingGame/Blueprints/FirstPersonHUD.Egg Get` true _asfirst_person_hud)))

(fn `UserConstructionScript`)