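; Trampoline actor that bounces the player character into the air when it is hit.
; A hit from a component named CollisionCylinder plays a sound, then launches player 0 along the actor's rotated up vector scaled by Force, plus the hit normal, overriding existing velocity.
; The same launch vector feeds a debug-drawn projectile path prediction from the hit location, which the G key also triggers on its own.
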(event `self.ReceiveHit`
  (params (MyComp :type "PrimitiveComponent Object Reference") (Other :type "Actor Object Reference") (OtherComp :type "PrimitiveComponent Object Reference") (bSelfMoved :type Boolean) (HitLocation :type "Vector Structure") (HitNormal :type "Vector Structure") (NormalImpulse :type "Vector Structure") (Hit :type "HitResult Structure (by ref)"))
  (bind _returnvalue (`GameplayStatics.GetPlayerCharacter` 0))
  (bind _force (`self.Force`))
  (bind _returnvalue_2 (+ HitNormal (* (`KismetMathLibrary.GetUpVector` (`self.K2_GetActorRotation`)) (`KismetMathLibrary.MakeVector` _force _force _force))))
  (if (`KismetStringLibrary.EqualEqual_StrStr` (`KismetStringLibrary.Conv_ObjectToString` OtherComp) "CollisionCylinder")
    (`GameplayStatics.SpawnSoundAtLocation` "/Game/AmazingGame/Audio/Trampoline.Trampoline" HitLocation (struct) 1.0 1.0 0.0 null null)
    (bind _assource_player_chracter (cast `/Game/AmazingGame/Blueprints/SourcePlayerChracter` _returnvalue))
    (`Character.LaunchCharacter` _assource_player_chracter _returnvalue_2 true true)
    (`GameplayStatics.Blueprint_PredictProjectilePath_ByTraceChannel` HitLocation _returnvalue_2 true 25.0 "ECC_Visibility" false (`|MakeArray` self _returnvalue :!type "Actor Object Reference") "ForDuration" 10.0 10.0 8.0 :!label _label)))

(event `Key|G` :consume false
  (params (Key :type "Key Structure"))
  (:`Pressed`
    (goto _label)))

(fn `UserConstructionScript`)